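; Checkpoint actor that saves a respawn transform when the 731Devatox character overlaps its Box trigger.
; It loads the existing 731SaveGame from the slot, or creates one if none exists.
; It stores the checkpoint's own location, raised along Z with zero rotation, rather than the player's transform, then saves to the slot.
; Each overlap saves again and shows a PopUpWidget_WB save notification.
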(event `self.Box.OnComponentBeginOverlap`
  (params (OverlappedComponent :type "PrimitiveComponent Object Reference") (OtherActor :type "Actor Object Reference") (OtherComp :type "PrimitiveComponent Object Reference") (OtherBodyIndex :type Integer) (bFromSweep :type Boolean) (SweepResult :type "HitResult Structure (by ref)"))
  (bind _returnvalue_location (`KismetMathLibrary.BreakTransform` (`self.GetTransform`)))
  (bind _as731devatox (cast `/Game/Blueprints/731Devatox` OtherActor))
  (set `self.As 731Devatox` _as731devatox)
  ;[0.1016 0.289 1] If a Save game file is not present then one gets created here
  (bind _returnvalue (`GameplayStatics.DoesSaveGameExist` (`self.Slot Name`)))
  (if _returnvalue
    (bind _returnvalue_2 (`GameplayStatics.LoadGameFromSlot` (`self.Slot Name`)))
    (bind _as731save_game (cast `/Game/Blueprints/Interactable/SAVE_SYSTEM/731SaveGame` _returnvalue_2))
    (set `self.SaveGameREF` _as731save_game)
    (else
      (bind _returnvalue_3 (`GameplayStatics.CreateSaveGameObject` "/Game/Blueprints/Interactable/SAVE_SYSTEM/731SaveGame.731SaveGame_C"))
      (set `self.SaveGameREF` _returnvalue_3)))
  ;[0.1016 0.289 1] This will save the players transform
  (set `/Game/Blueprints/Interactable/SAVE_SYSTEM/731SaveGame.Checkpoint` (`KismetMathLibrary.MakeTransform` (+ _returnvalue_location (0.0 0.0 200.0))) (`self.SaveGameREF`))
  (`GameplayStatics.SaveGameToSlot` (`self.SaveGameREF`) (`self.Slot Name`))
  ;[0.1016 0.289 1] Creates a save notification pop up widget
  (bind _returnvalue_4 (`|CreateWidget` "/Game/Blueprints/UI/PopUpWidget_WB.PopUpWidget_WB_C"))
  (`/Game/Blueprints/UI/PopUpWidget_WB.SaveNotification` _returnvalue_4)
  (`UserWidget.AddToViewport` _returnvalue_4 0))

(fn `UserConstructionScript`)